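; Main game mode that handles restarts by respawning level actors and repositioning the player.
; On BeginPlay it binds a restart event, which calls SpawnActor on every Bp_ActorSpawner in the level.
; The event then moves the player character to the SpawnLocation stored in DropperGameInstance, if that location is non-zero.
; A level-loaded notification to the game instance is present but disconnected, so it never runs.
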(event Custom|Restart_Event
  (bind _outactors (Actor|GetAllActorsOfClass "/Game/Bp_ActorSpawner.Bp_ActorSpawner_C"))
  (for _array_element _outactors
    (Class|CollectableSpawner|SpawnActor _array_element))
  (bind _asdropper_game_instance (Utilities|Casting|CastToDropperGameInstance (Game|GetGameInstance)))
  (Utilities|FlowControl|Sequence
    (:then_0
      (if (Utilities|Operators|NotEqual(!=) :A (Variables|/Script/CharacterProject.DropperGameInstance|GetSpawnLocation _asdropper_game_instance))
        (Transformation|SetActorLocation (Game|GetPlayerCharacter 0) (Variables|/Script/CharacterProject.DropperGameInstance|GetSpawnLocation _asdropper_game_instance) false false)))))

(event EventBeginPlay
  (EventDispatchers|BindEventtoRestart (delegate Custom|Restart_Event)))

(fn ConstructionScript)