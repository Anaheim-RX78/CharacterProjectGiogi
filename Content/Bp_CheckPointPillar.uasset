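; Checkpoint pillar for a dropper game that records a new spawn location for the player when activated.
; Its OpenDoor event turns the pillar solid blue, reveals the Scene component with its children and hides the text label.
; It then writes the CheckPoint component's world location to SpawnLocation on the DropperGameInstance.
; Nothing in this Blueprint triggers the event itself.
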(event EventOpenDoor
  (Rendering|Material|SetMaterial (Variables|Default|GetPillar) 0 "/Game/LevelPrototyping/Materials/MI_Solid_Blue.MI_Solid_Blue")
  (Rendering|SetVisibility (Variables|Default|GetScene) true true)
  (Rendering|SetVisibility (Variables|Default|GetTextRender) false false)
  (bind _asdropper_game_instance (Utilities|Casting|CastToDropperGameInstance (Game|GetGameInstance)))
  (Variables|/Script/CharacterProject.DropperGameInstance|SetSpawnLocation _asdropper_game_instance (Transformation|GetWorldLocation (Variables|Default|GetCheckPoint))))

(fn ConstructionScript)