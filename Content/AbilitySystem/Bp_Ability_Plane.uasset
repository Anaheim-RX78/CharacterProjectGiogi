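; Bp_Ability_Plane is an ability actor that lowers the movement speed multiplier of the owning Bp_PinkoCharacter to 0.9 while it is active.
; On BeginPlay it waits a tick and caches the owner, and Tick then reapplies the multiplier every frame.
; After the duration from AbilityData it resets the multiplier to 1.0, without restoring any earlier value, and destroys itself.
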(event EventBeginPlay
  (Utilities|FlowControl|DelayUntilNextTick)
  (bind _asbp_pinko_character (Utilities|Casting|CastToBp_PinkoCharacter (Variables|Default|GetOwnerCharacter)))
  (Variables|Default|SetAs%20Bp%20Pinko%20Character _asbp_pinko_character)
  (Utilities|FlowControl|Delay (Variables|/Script/CharacterProject.AbilityData|GetDuration (Variables|Default|GetAbilityData)))
  (Variables|/Script/CharacterProject.Pinko|SetMovementSpeedMultiplier (Variables|Default|GetAs%20Bp%20Pinko%20Character) 1.0)
  (Actor|DestroyActor))

(event EventTick
  (params (DeltaSeconds :type Float%20%28single-precision%29))
  (bind _as_bp_pinko_character (Variables|Default|GetAs%20Bp%20Pinko%20Character)
    (:then
      (Variables|/Script/CharacterProject.Pinko|SetMovementSpeedMultiplier _as_bp_pinko_character 0.9))
    (:else)))

(fn ConstructionScript)