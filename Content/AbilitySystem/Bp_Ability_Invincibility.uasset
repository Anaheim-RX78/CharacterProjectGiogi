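; Timed invincibility ability actor that makes its owning Pinko character invincible and turns it white.
; On BeginPlay it waits a tick, casts the owner, sets the invincible flag and caches the mesh's materials before replacing every slot with a white material instance.
; After the duration from the ability data, it clears the flag, restores the cached materials and destroys itself.
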(event EventBeginPlay
  (Utilities|FlowControl|DelayUntilNextTick)
  (bind _asbp_pinko_character (Utilities|Casting|CastToBp_PinkoCharacter (Variables|Default|GetOwnerCharacter)))
  (bind _output_get (Variables|Default|SetAs%20Bp%20Pinko%20Character _asbp_pinko_character))
  (Variables|/Script/CharacterProject.Pinko|SetIsInvincible _output_get true)
  (CallFunction|SetMaterials true "/Game/Collectables/Materials/MI_Color_White.MI_Color_White")
  (Utilities|FlowControl|Delay (Variables|/Script/CharacterProject.AbilityData|GetDuration (Variables|Default|GetAbilityData)))
  (Variables|/Script/CharacterProject.Pinko|SetIsInvincible (Variables|Default|GetAs%20Bp%20Pinko%20Character) false)
  (CallFunction|SetMaterials false "/Game/Collectables/Materials/MI_Color_White.MI_Color_White")
  (Actor|DestroyActor))

(fn ConstructionScript)

(fn SetMaterials
  (params (UseNew :type Boolean) (NewMaterial :type Material%20Interface%20Object%20Reference))
  (if UseNew
    (Utilities|Array|Clear (Variables|Default|GetCharacter%20Materials))
    (bind _output_get (Variables|Default|SetCharacter%20Materials (Rendering|Material|GetMaterials (Variables|/Script/Engine.Character|GetMesh (Variables|Default|GetAs%20Bp%20Pinko%20Character)))))
    (for (_ _array_index) _output_get
      (Rendering|Material|SetMaterial (Variables|/Script/Engine.Character|GetMesh (Variables|Default|GetAs%20Bp%20Pinko%20Character)) _array_index NewMaterial))
    (else
      (for (_array_element _array_index_2) (Variables|Default|GetCharacter%20Materials)
        (Rendering|Material|SetMaterial (Variables|/Script/Engine.Character|GetMesh (Variables|Default|GetAs%20Bp%20Pinko%20Character)) _array_index_2 _array_element)))))