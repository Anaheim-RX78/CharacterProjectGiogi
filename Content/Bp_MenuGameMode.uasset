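; Menu game mode that prepares UI-only input with a visible cursor and handles level switching.
; On BeginPlay it caches the DropperGameInstance and stores the current level name in it as the level identifier, stopping if the cast fails.
; Its OpenLevel event notifies the game instance through OnLevelLoaded before opening the requested level by name.
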(event Custom|OpenLevel
  (params (Level :type String))
  (Class|DropperGameInstance|OnLevelLoaded (Variables|Default|GetAs%20Dropper%20Game%20Instance) Level)
  (Game|OpenLevel(byName) (Utilities|String|StringToName Level)))

(event EventBeginPlay
  (bind _returnvalue (Game|GetPlayerController 0))
  (bind _asdropper_game_instance (Utilities|Casting|CastToDropperGameInstance (Game|GetGameInstance)))
  (bind _output_get (Variables|Default|SetAs%20Dropper%20Game%20Instance _asdropper_game_instance))
  (bind _returnvalue_2 (Game|GetCurrentLevelName true))
  (Variables|/Script/CharacterProject.DropperGameInstance|SetCurrentLevelIdentifier _output_get _returnvalue_2)
  (Input|SetInputModeUIOnly _returnvalue 0 "DoNotLock" false)
  (Variables|/Script/Engine.PlayerController|SetbShowMouseCursor _returnvalue true))

(fn ConstructionScript)